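; Player character Blueprint that handles Enhanced Input for looking, moving and jumping.
; BeginPlay adds the IMP_Player mapping context through the PC_Player controller's local player subsystem.
; Movement follows control-rotation yaw only, while look input drives controller pitch and yaw.
; CanLook, CanMove and CanJump flags gate these actions and are set together by TogglePlayerLocks.
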(event `self.ReceiveBeginPlay`
  (bind _aspc_player (cast `/Game/Blueprints/Player/PC_Player` (`GameplayStatics.GetPlayerController` 0)))
  (`EnhancedInputSubsystemInterface.AddMappingContext` (pcsubsystem `EnhancedInputLocalPlayerSubsystem` _aspc_player) "/Game/Input/IMP_Player.IMP_Player" 0 (struct)))

(event `EnhancedInput|/Game/Input/IA_Look`
  (params (ActionValue :type "Vector2D Structure") (ElapsedSeconds :type "Float (double-precision)") (TriggeredSeconds :type "Float (double-precision)") (InputAction :type "InputAction Object Reference" :default "/Game/Input/IA_Look.IA_Look"))
  (:`Triggered`
    (if (`self.CanLook?`)
      (bind _result (`/Engine/EditorBlueprintResources/StandardMacros.NegateFloat` ActionValue_Y)
        (:`  `
          (`self.AddControllerPitchInput` _result)
          (`self.AddControllerYawInput` ActionValue_X))))))

(event `EnhancedInput|/Game/Input/IA_MoveForward`
  (params (ActionValue :type "Float (double-precision)") (ElapsedSeconds :type "Float (double-precision)") (TriggeredSeconds :type "Float (double-precision)") (InputAction :type "InputAction Object Reference" :default "/Game/Input/IA_MoveForward.IA_MoveForward"))
  (:`Triggered`
    (if (`self.CanMove?`)
      (`self.AddMovementInput` (`KismetMathLibrary.GetForwardVector` (`KismetMathLibrary.MakeRotator` 0.0 0.0 (.yaw (`self.GetControlRotation`)))) ActionValue))))

(event `EnhancedInput|/Game/Input/IA_MoveRight`
  (params (ActionValue :type "Float (double-precision)") (ElapsedSeconds :type "Float (double-precision)") (TriggeredSeconds :type "Float (double-precision)") (InputAction :type "InputAction Object Reference" :default "/Game/Input/IA_MoveRight.IA_MoveRight"))
  (:`Triggered`
    (if (`self.CanMove?`)
      (`self.AddMovementInput` (`KismetMathLibrary.GetRightVector` (`KismetMathLibrary.MakeRotator` 0.0 0.0 (.yaw (`self.GetControlRotation`)))) ActionValue))))

(event `EnhancedInput|/Game/Input/IA_Jump`
  (params (ActionValue :type Boolean) (ElapsedSeconds :type "Float (double-precision)") (TriggeredSeconds :type "Float (double-precision)") (InputAction :type "InputAction Object Reference" :default "/Game/Input/IA_Jump.IA_Jump"))
  (:`Started`
    (if (`self.CanJump?`)
      (`self.Jump`)))
  (:`Completed`
    (`self.StopJumping`)))

(fn `Toggle PlayerLocks`
  (params (Look :type Boolean) (Move :type Boolean) (Jump :type Boolean))
  (set `self.CanLook?` Look)
  (set `self.CanMove?` Move)
  (set `self.CanJump?` Jump))

(fn `UserConstructionScript`)
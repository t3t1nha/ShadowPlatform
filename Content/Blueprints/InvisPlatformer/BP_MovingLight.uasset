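; BP_MovingLight is an actor in the InvisPlatformer folder that moves a spot light back and forth along a spline path.
; BeginPlay caches the spline length, then Tick advances a clamped distance by speed, direction and delta time.
; The direction flips at either end of the spline.
; On other frames, the light is placed at the world location for that distance, with no rotation change.
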(event `self.ReceiveBeginPlay`
  (set `self.SplineLength` (`SplineComponent.GetSplineLength` (`self.LightPath`))))

(event `self.ReceiveTick`
  (params (DeltaSeconds :type "Float (single-precision)"))
  (bind _splinelength (`self.SplineLength`))
  (bind _current_spline_location (`self.Current Spline Location`))
  (set `self.Current Spline Location` (`KismetMathLibrary.FClamp` (+ (`self.Current Spline Location`) (* (`self.Direction`) DeltaSeconds (`self.Speed`))) 0.0 (`self.SplineLength`)))
  (if (>= _current_spline_location _splinelength)
    (set `self.Current Spline Location` _splinelength)
    (set `self.Direction` -1.0)
    (elif (<= _current_spline_location 0.0)
      (set `self.Current Spline Location` 0.0)
      (set `self.Direction` 1.0)
      (else
        (`SceneComponent.K2_SetWorldLocation` (`self.SpotLight`) (`SplineComponent.GetLocationAtDistanceAlongSpline` (`self.LightPath`) (`self.Current Spline Location`) "World") false false)))))

(fn `UserConstructionScript`)